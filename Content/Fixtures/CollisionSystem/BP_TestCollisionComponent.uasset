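; Test collision component that sweeps sphere traces along the socket paths of registered meshes to detect hits.
; While tracing is enabled, each tick traces from every socket's cached previous location to its current one, after a first tick that only caches locations.
; Hits skip the owner, already-hit actors and ignored collision profiles or classes (only the first class entry is checked), then fire OnHitRegistered.
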(event EventBeginPlay
  (Default|CallOnComponentBeginPlay))

(event EventTick
  (params (DeltaSeconds :type Float%20%28single-precision%29))
  (if (Variables|Default|GetbCanTrace)
    (Development|PrintString "Collision Tick" true false "(R=0.000000,G=0.660000,B=1.000000,A=1.000000)" 0.0)
    (CallFunction|TraceTick)
    (else
      (Development|PrintString "Collision Not Tick" true false "(R=0.000000,G=0.660000,B=1.000000,A=1.000000)" 0.0))))

(event EventEndPlay
  (params (EndPlayReason :type EEndPlayReason%20Enum :default "Destroyed"))
  (Default|CallOnComponentEndPlay EndPlayReason))

(fn StartTrace
  (Variables|Default|SetbCanTrace true)
  (CallFunction|ResetHitActors)
  (Default|CallOnTraceStart))

(fn EndTrace
  (Variables|Default|SetbCanTrace false)
  (Variables|Default|SetbIsTraceRunning false)
  (Default|CallOnTraceEnd))

(fn RegisterCollisionMesh
  (params (InMesh :type Primitive%20Component%20Object%20Reference%20%28by%20ref%29))
  (Utilities|Array|AddUnique (Variables|Default|GetCollisionPrimitiveComponents) InMesh))

(fn UnregisterCollisionMesh
  (params (InMesh :type Primitive%20Component%20Object%20Reference%20%28by%20ref%29))
  (Utilities|Array|RemoveItem (Variables|Default|GetCollisionPrimitiveComponents) InMesh))

(fn TraceTick
  (if (Variables|Default|GetbIsTraceRunning) ; First tick, just update socket locations so \non next tick it will be able to compare socket locations
    (CallFunction|DoTraceCheckforRegisteredMeshes))
  (CallFunction|UpdateSocketLocations)
  (Variables|Default|SetbIsTraceRunning true))

(fn UpdateSocketLocations
  (for _array_element (Variables|Default|GetCollisionPrimitiveComponents)
    (for _array_element_2 (Transformation|GetAllSocketNames _array_element)
      (Utilities|Map|Add (Variables|Default|GetLastFrameSocketLocations) (CallFunction|GenerateUniqueSocketName _array_element _array_element_2) (Transformation|GetSocketLocation _array_element _array_element_2)))))

(fn GenerateUniqueSocketName
  (params (InMesh :type Primitive%20Component%20Object%20Reference) (InSocketName :type Name))
  (Utilities|IsValid InMesh
    (:Is%20Valid
      (return (Utilities|String|StringToName (Utilities|String|Append (Utilities|GetObjectName InMesh) "." (Utilities|String|ToString(Name) InSocketName)))))
    (:Is%20Not%20Valid
      (return "None"))))

(fn DoTraceCheckforRegisteredMeshes
  (for _array_element (Variables|Default|GetCollisionPrimitiveComponents)
    (for _array_element_2 (Transformation|GetAllSocketNames _array_element)
      (CallFunction|DoTraceCheckforSocket _array_element _array_element_2))))

(fn DoTraceCheckforSocket
  (params (InMesh :type Primitive%20Component%20Object%20Reference) (SocketName :type Name))
  ;[0 0.2734 1] Calculate Previous / Current Socket location for trace
  (LocalVariables|SetPreviousSocketLocation (.Value (Utilities|Map|Find (Variables|Default|GetLastFrameSocketLocations) (CallFunction|GenerateUniqueSocketName InMesh SocketName))))
  (LocalVariables|SetCurrentSocketLocation (Transformation|GetSocketLocation InMesh SocketName))
  ;[1 0 0.9375] Perform Trace by Channel
  (bind (_outhits _returnvalue) (Collision|MultiSphereTraceByChannel (LocalVariables|GetPreviousSocketLocation) (LocalVariables|GetCurrentSocketLocation) (Variables|Default|GetTraceRadius) (Variables|Default|GetCollisionTraceChannel) false (Variables|Default|GetHitActors) (select (Variables|Default|GetbDebug) "ForDuration" "None")))
  (if _returnvalue
    (for _array_element _outhits
      (if (Math|Boolean|ANDBoolean (not (Utilities|Array|ContainsItem (Variables|Default|GetHitActors) (.HitActor (Collision|BreakHitResult _array_element)))) (not (CallFunction|IsIgnoredClass (Utilities|GetClass (.HitActor (Collision|BreakHitResult _array_element))))) (not (Utilities|Array|ContainsItem (Variables|Default|GetIgnoredProfileNames) (Collision|GetCollisionProfileName (.HitComponent (Collision|BreakHitResult _array_element))))))
        (CallFunction|HandleSuccessfulHit _array_element InMesh)))))

(fn ResetHitActors
  (Utilities|Array|Clear (Variables|Default|GetHitActors))
  (Utilities|Array|Add (Variables|Default|GetHitActors) (Components|GetOwner)))

(fn IsIgnoredClass
  (params (InClass :type Actor%20Class%20Reference))
  (bind _array_element (Utilities|Array|ForEachLoopwithBreak (Variables|Default|GetIgnoredClasses) :!label _label)
    (:LoopBody
      (if true
        (LocalVariables|SetbIsIgnored (Utilities|ClassIsChildOf InClass _array_element))
        (goto _label Break)))
    (:Completed
      (return (LocalVariables|GetbIsIgnored)))))

(fn HandleSuccessfulHit
  (params (InHitResult :type Hit%20Result%20Structure) (InMesh :type Primitive%20Component%20Object%20Reference))
  (Utilities|Array|Add (Variables|Default|GetHitActors) (.HitActor (Collision|BreakHitResult InHitResult)))
  (Default|CallOnHitRegistered InHitResult InMesh))